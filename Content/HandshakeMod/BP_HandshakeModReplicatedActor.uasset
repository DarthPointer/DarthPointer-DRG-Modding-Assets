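; Per-player replicated actor that handshakes mod IDs registered on a client with their hostside counterparts.
; Locally, it drains the clientside storage asset, listens for new registrations and forwards IDs through server events.
; The host side passes IDs and the owning PlayerController to HostsideMasterActor, retrying when a matching hostside mod registers later.
; A hub page widget lists local mods and shows debug messages.
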(event EventBeginPlay
  (CallFunction|HandleBeginPlay))

(event Collision|EventActorBeginOverlap
  (params (OtherActor :type Actor%20Object%20Reference))
  (|CallParentFunction OtherActor) ; This node is disabled and will not be called.\nDrag off pins to build functionality.
)

(event EventTick
  (params (DeltaSeconds :type Float%20%28single-precision%29))
  (|CallParentFunction DeltaSeconds) ; This node is disabled and will not be called.\nDrag off pins to build functionality.
)

(event Custom|Server%20Recieve%20Clientside%20Mod%20Registered
  (params (Mod%20ID :type String))
  (CallFunction|ServersideProcessRegisteredClientsideMod Mod%20ID))

(event Custom|Server%20Process%20All%20Currently%20Registered%20Mods
  (CallFunction|ServersideProcessAllCurrentlyRegisteredMods))

(fn ConstructionScript
  (|CallParentFunction))

(fn HandleBeginPlay
  (bind _returnvalue (UserInterface|CreateWidget "/Game/HandshakeMod/UI_HandshakeModHubPage.UI_HandshakeModHubPage_C"))
  (bind _output_get (Variables|Default|SetMod%20Hub%20Page _returnvalue))
  (CallFunction|AddPage _output_get)
  (Utilities|FlowControl|Sequence
    (:then_0
      (if (Networking|IsServer)
        (CallFunction|HostsideInit)))
    (:then_1
      (if (Pawn|IsLocalPlayerController (Variables|Default|GetOwning%20Player%20Controller))
        (CallFunction|ClientsideInit)))))

(fn ClientsideInit
  (bind _clientside_registered_mods_storage_asset (Variables|Default|GetClientside%20Registered%20Mods%20Storage%20Asset))
  (bind _registered_mods_ids (Variables|/Game/HandshakeMod/BP_ClientsideRegisteredModsStorage.BP_ClientsideRegisteredModsStorage_C|GetRegistered%20Mods%20IDs _clientside_registered_mods_storage_asset))
  (Variables|Default|SetRegistered%20Clientside%20Mods%20IDs _registered_mods_ids)
  (Utilities|Array|Clear _registered_mods_ids)
  (Default|DisplayLocallyRegisteredModsIDs (Variables|Default|GetMod%20Hub%20Page) (Variables|Default|GetRegistered%20Clientside%20Mods%20IDs))
  (CallFunction|ServerProcessAllCurrentlyRegisteredMods)
  (EventDispatchers|BindEventtoOnLocalModRegistered _clientside_registered_mods_storage_asset (EventDispatchers|CreateEvent :!event HandleonLocalModRegistered)))

(fn HandleonLocalModRegistered
  (params (Mod%20ID :type String))
  (Utilities|Array|AddUnique (Variables|Default|GetRegistered%20Clientside%20Mods%20IDs) Mod%20ID)
  (Utilities|Array|Clear (Variables|/Game/HandshakeMod/BP_ClientsideRegisteredModsStorage.BP_ClientsideRegisteredModsStorage_C|GetRegistered%20Mods%20IDs (Variables|Default|GetClientside%20Registered%20Mods%20Storage%20Asset)))
  (Default|DisplayLocallyRegisteredModsIDs (Variables|Default|GetMod%20Hub%20Page) (Variables|Default|GetRegistered%20Clientside%20Mods%20IDs))
  (CallFunction|ServerRecieveClientsideModRegistered Mod%20ID))

(fn ServersideProcessRegisteredClientsideMod
  (params (Mod%20ID :type String))
  (Default|TryNotifyHostsideMod (Variables|Default|GetHostside%20Master%20Actor) Mod%20ID (Variables|Default|GetOwning%20Player%20Controller)))

(fn ServersideProcessAllCurrentlyRegisteredMods
  (for _array_element (Variables|Default|GetRegistered%20Clientside%20Mods%20IDs)
    (CallFunction|ServersideProcessRegisteredClientsideMod _array_element)))

(fn HostsideInit
  (|CollapseGraph_0)
  (EventDispatchers|BindEventtoOnHostsideModRegistered (Variables|Default|GetHostside%20Master%20Actor) (EventDispatchers|CreateEvent :!event HandleonHostsideModRegistered)))

(fn HandleonHostsideModRegistered
  (params (Mod%20ID :type String))
  (|CollapseGraph_0_2 Mod%20ID)
  (if (Utilities|Array|ContainsItem (Variables|Default|GetRegistered%20Clientside%20Mods%20IDs) Mod%20ID)
    (|CollapseGraph_0_3 Mod%20ID)
    (CallFunction|ServersideProcessRegisteredClientsideMod Mod%20ID)))