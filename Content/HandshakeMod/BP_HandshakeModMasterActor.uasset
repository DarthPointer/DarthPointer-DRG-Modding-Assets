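; Server-side master actor for the Handshake mod, linking host-registered mods to players' controllers.
; On BeginPlay it adds a hub debug page, listens to the shared mod storage and spawns an owned replicated actor per current player, binding the login event.
; New registrations move from storage into its mod-ID map and are rebroadcast.
; TryNotifyHostsideMod looks up an ID and passes that client's controller to the matching mod, logging to the page.
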(event EventBeginPlay
  (CallFunction|HandleBeginPlay))

(event Collision|EventActorBeginOverlap
  (params (OtherActor :type Actor%20Object%20Reference))
  (|CallParentFunction OtherActor) ; This node is disabled and will not be called.\nDrag off pins to build functionality.
)

(event EventTick
  (params (DeltaSeconds :type Float%20%28single-precision%29))
  (|CallParentFunction DeltaSeconds) ; This node is disabled and will not be called.\nDrag off pins to build functionality.
)

(fn ConstructionScript
  (|CallParentFunction))

(fn HandleBeginPlay
  (bind _hostside_listening_mods_storage (Variables|Default|GetHostside%20Listening%20Mods%20Storage))
  (if (Networking|IsServer)
    (bind _returnvalue (UserInterface|CreateWidget "/Game/HandshakeMod/UI_HandshakeModHubPage.UI_HandshakeModHubPage_C"))
    (bind _output_get (Variables|Default|SetMod%20Hub%20Page _returnvalue))
    (CallFunction|AddPage _output_get)
    (Variables|Default|SetFSD%20Game%20Mode (Class|GameFunctionLibrary|GetFSDGameMode self))
    (bind _output_get_2 (Variables|Default|SetHandshake%20Awaiting%20Mods (Variables|/Game/HandshakeMod/BP_HostsideListeningModsStorage.BP_HostsideListeningModsStorage_C|GetHandshake%20Awaiting%20Mods _hostside_listening_mods_storage)))
    (Utilities|Map|Clear _output_get_2)
    (bind _keys (Utilities|Map|Keys (Variables|Default|GetHandshake%20Awaiting%20Mods)))
    (Default|DisplayLocallyRegisteredModsIDs (Variables|Default|GetMod%20Hub%20Page) _keys)
    (EventDispatchers|BindEventtoOnHostsideModRegistered _hostside_listening_mods_storage (EventDispatchers|CreateEvent :!event HandleonHostsideModRegistered))
    (for _array_element (Variables|/Script/FSD.FSDGameMode|GetPlayerControllers (Variables|Default|GetFSD%20Game%20Mode))
      (CallFunction|SpawnReplicatedActorforPlayer _array_element))
    (EventDispatchers|BindEventtoOnPlayerLoggedin (Variables|Default|GetFSD%20Game%20Mode) (EventDispatchers|CreateEvent :!event SpawnReplicatedActorforPlayer))))

(fn SpawnReplicatedActorforPlayer
  (params (FSD%20Player%20Controller :type FSD%20Player%20Controller%20Object%20Reference))
  (Game|SpawnActorfromClass "/Game/HandshakeMod/BP_HandshakeModReplicatedActor.BP_HandshakeModReplicatedActor_C" (Math|Transform|MakeTransform "0, 0, 0") "Undefined" FSD%20Player%20Controller self FSD%20Player%20Controller 0))

(fn HandleonHostsideModRegistered
  (params (Mod%20ID :type String) (Handshake%20Awaiting%20Mod :type I%20Handshake%20Awaiting%20Object%20Interface))
  (|CollapseGraph_0 Mod%20ID)
  (Utilities|Map|Add (Variables|Default|GetHandshake%20Awaiting%20Mods) Mod%20ID Handshake%20Awaiting%20Mod)
  (Utilities|Map|Clear (Variables|/Game/HandshakeMod/BP_HostsideListeningModsStorage.BP_HostsideListeningModsStorage_C|GetHandshake%20Awaiting%20Mods (Variables|Default|GetHostside%20Listening%20Mods%20Storage)))
  (bind _keys (Utilities|Map|Keys (Variables|Default|GetHandshake%20Awaiting%20Mods)))
  (Default|DisplayLocallyRegisteredModsIDs (Variables|Default|GetMod%20Hub%20Page) _keys)
  (Default|CallOnHostsideModRegistered Mod%20ID))

(fn TryNotifyHostsideMod
  (params (Mod%20ID :type String) (Clientside%20Owned%20Player%20Controller :type FSD%20Player%20Controller%20Object%20Reference))
  (bind _handshake_awaiting_mods (Variables|Default|GetHandshake%20Awaiting%20Mods))
  (bind (_value _returnvalue) (Utilities|Map|Find _handshake_awaiting_mods Mod%20ID))
  (|CollapseGraph_0_2 Mod%20ID)
  (if _returnvalue
    (|CollapseGraph_0_3 Mod%20ID)
    (Default|OnModRegisteredforPlayerController _value Clientside%20Owned%20Player%20Controller)))