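; BP_VanityModArmorItem is a vanity mod armor item that registers itself with the vanity sets of Driller, Engineer, Gunner and Scout.
; AddItem checks each class flag in sequence and calls AddforSet, which appends the item to that set's ArmorItems array.
; The Driller branch calls AddforSet twice on the same set, unlike the other three classes.
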(event EventAddforSet
  (params (Vanity%20Set :type Character%20Vanity%20Items%20Object%20Reference))
  (Utilities|Array|Add (Variables|/Script/FSD.CharacterVanityItems|GetArmorItems Vanity%20Set) self))

(event EventAddItem
  (Utilities|FlowControl|Sequence
    (:then_0
      (if (Variables|VanityMod|GetDriller)
        (CallFunction|AddforSet "/Game/Character/Vanity2/_VanitySets/VanitySet_Driller.VanitySet_Driller")
        (CallFunction|AddforSet "/Game/Character/Vanity2/_VanitySets/VanitySet_Driller.VanitySet_Driller")))
    (:then_1
      (if (Variables|VanityMod|GetEngineer)
        (CallFunction|AddforSet "/Game/Character/Vanity2/_VanitySets/VanitySet_Engineer.VanitySet_Engineer")))
    (:then_2
      (if (Variables|VanityMod|GetGunner)
        (CallFunction|AddforSet "/Game/Character/Vanity2/_VanitySets/VanitySet_Gunner.VanitySet_Gunner")))
    (:then_3
      (if (Variables|VanityMod|GetScout)
        (CallFunction|AddforSet "/Game/Character/Vanity2/_VanitySets/VanitySet_Scout.VanitySet_Scout")))))