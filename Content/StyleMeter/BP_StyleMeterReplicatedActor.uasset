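; Replicated actor for the Style Meter mod that sets up the style HUD and its Mod Hub settings page for the local player.
; On BeginPlay the local client loads or creates a config save, builds both widgets from it, and retries on a looping timer until widgets are ready for the viewport.
; Settings events update config and HUD live, with separate mission and Space Rig visibility saved immediately.
; Host-side init is an empty stub.
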(event EventBeginPlay
  (CallFunction|HandleBeginPlay))

(event Collision|EventActorBeginOverlap
  (params (OtherActor :type Actor%20Object%20Reference))
  (|CallParentFunction OtherActor) ; This node is disabled and will not be called.\nDrag off pins to build functionality.
)

(event EventTick
  (params (DeltaSeconds :type Float%20%28single-precision%29))
  (|CallParentFunction DeltaSeconds) ; This node is disabled and will not be called.\nDrag off pins to build functionality.
)

(fn ConstructionScript
  (|CallParentFunction))

(fn HandleBeginPlay
  (Utilities|FlowControl|Sequence
    (:then_0
      (if (Networking|IsServer)
        (CallFunction|HostsideInit)))
    (:then_1
      (if (Pawn|IsLocalPlayerController (Variables|Default|GetOwning%20Controller))
        (CallFunction|ClientsideInit)))))

(fn ClientsideInit
  (ConfigSaveLoading|LoadConfig)
  (CallFunction|CreateandSetupStyleHUD)
  (CallFunction|AddHUDstoViewportOnceWidgetsAreReady)
  (CallFunction|CreateandSetupModHubSettingsPage))

(fn HostsideInit)

(fn GetModInfo
  (return "Style Meter" "Darth Pointer" "0.0.0"))

(fn CreateandSetupModHubPage)

(fn LoadConfig
  (bind _returnvalue (SaveGame|LoadGamefromSlot (Variables|Default|GetConfig%20Save%20Name)))
  (Utilities|IsValid _returnvalue
    (:Is%20Valid
      (bind _assav_style_meter_config (Utilities|Casting|CastToSAV_StyleMeterConfig _returnvalue)
        (:then
          (Variables|Default|SetConfig _assav_style_meter_config))
        (:CastFailed
          (bind _returnvalue_2 (SaveGame|CreateSaveGameObject "/Game/StyleMeter/SAV_StyleMeterConfig.SAV_StyleMeterConfig_C" :!label _label))
          (Variables|Default|SetConfig _returnvalue_2))))
    (:Is%20Not%20Valid
      (goto _label))))

(fn SaveConfig
  (SaveGame|SaveGametoSlot (Variables|Default|GetConfig) (Variables|Default|GetConfig%20Save%20Name)))

(fn CreateandSetupModHubSettingsPage
  (bind _returnvalue (UserInterface|CreateWidget "/Game/StyleMeter/UI_StyleMeterModHubPage.UI_StyleMeterModHubPage_C"))
  (bind _output_get (Variables|Default|SetMod%20Hub%20Settings%20Page _returnvalue))
  (CallFunction|AddPage _output_get)
  (Default|SetupfromConfig _output_get (Variables|Default|GetConfig))
  (|ModHubPageEventsSubscribtions))

(fn CreateandSetupStyleHUD
  (bind _returnvalue (UserInterface|CreateWidget "/Game/StyleMeter/UI_StyleHUD.UI_StyleHUD_C"))
  (bind _output_get (Variables|Default|SetStyle%20HUD _returnvalue))
  (Default|ApplyGameHUDVisible _output_get (Class|FSDWidgetBlueprintLibrary|IsHUDVisible self))
  (EventDispatchers|BindEventtoOnHUDVisibilityChanged (Class|FSDHUD|GetFSDHUD (Variables|Default|GetOwning%20Controller)) (EventDispatchers|CreateEvent (Variables|Default|GetStyle%20HUD) :!event ApplyGameHUDVisible))
  (Default|ApplyVisibleinCurrentScene (Variables|Default|GetStyle%20HUD) (CallFunction|IsHUDVisibleinCurrentScene))
  (Default|SetupfromConfig (Variables|Default|GetStyle%20HUD) (Variables|Default|GetConfig)))

(fn AddHUDstoViewportOnceWidgetsAreReady
  (bind _returnvalue (Utilities|Time|SetTimerbyEvent (EventDispatchers|CreateEvent :!event TryAddHUDstoViewport) 0.5 true))
  (Variables|Default|SetWidgets%20Ready%20Retrial%20Timer%20Handle _returnvalue))

(fn TryAddHUDstoViewport
  (if (CallFunction|WidgetsAreReady)
    (Utilities|Time|ClearandInvalidateTimerbyHandle (Variables|Default|GetWidgets%20Ready%20Retrial%20Timer%20Handle))
    (UserInterface|Viewport|AddtoViewport (Variables|Default|GetStyle%20HUD) 0)))

(fn InputDisplayStyleHUDinMission
  (params (Display :type Boolean))
  (Variables|/Game/StyleMeter/SAV_StyleMeterConfig.SAV_StyleMeterConfig_C|SetDisplay%20Style%20HUD%20In%20Mission (Variables|Default|GetConfig) Display)
  (ConfigSaveLoading|SaveConfig)
  (Default|ApplyVisibleinCurrentScene (Variables|Default|GetStyle%20HUD) (CallFunction|IsHUDVisibleinCurrentScene)))

(fn InputDisplayStyleHUDonSpacerig
  (params (Display :type Boolean))
  (Variables|/Game/StyleMeter/SAV_StyleMeterConfig.SAV_StyleMeterConfig_C|SetDisplay%20Style%20HUD%20On%20Spacerig (Variables|Default|GetConfig) Display)
  (ConfigSaveLoading|SaveConfig)
  (Default|ApplyVisibleinCurrentScene (Variables|Default|GetStyle%20HUD) (CallFunction|IsHUDVisibleinCurrentScene)))

(fn InputStyleHUDHorisontalPosition
  (params (Position :type Float%20%28single-precision%29))
  (Variables|/Game/StyleMeter/SAV_StyleMeterConfig.SAV_StyleMeterConfig_C|SetStyle%20HUD%20Horisontal%20Position (Variables|Default|GetConfig) Position)
  (Default|ApplyHorisontalPosition (Variables|Default|GetStyle%20HUD) Position))

(fn InputStyleHUDVerticalPosition
  (params (Position :type Float%20%28single-precision%29))
  (Variables|/Game/StyleMeter/SAV_StyleMeterConfig.SAV_StyleMeterConfig_C|SetStyle%20HUD%20Vertical%20Position (Variables|Default|GetConfig) Position)
  (Default|ApplyVerticalPosition (Variables|Default|GetStyle%20HUD) Position))

(fn IsHUDVisibleinCurrentScene
  (bind _config (Variables|Default|GetConfig))
  (return (select (CallFunction|IsonSpacerig) (Variables|/Game/StyleMeter/SAV_StyleMeterConfig.SAV_StyleMeterConfig_C|GetDisplay%20Style%20HUD%20On%20Spacerig _config) (Variables|/Game/StyleMeter/SAV_StyleMeterConfig.SAV_StyleMeterConfig_C|GetDisplay%20Style%20HUD%20In%20Mission _config))))