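; BP_StyleMeterMasterActor is the manager actor for the style meter, creating a BP_StyleMeterReplicatedActor for player controllers.
; On BeginPlay it spawns one for each controller in the FSD game mode and binds an event to the game mode's player-logged-in delegate.
; Each spawned actor is owned by its controller and receives references to that controller and to this master actor.
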(event EventBeginPlay
  (CallFunction|HandleBeginPlay))

(event Collision|EventActorBeginOverlap
  (params (OtherActor :type Actor%20Object%20Reference)))

(event EventTick
  (params (DeltaSeconds :type Float%20%28single-precision%29)))

(fn ConstructionScript)

(fn HandleBeginPlay
  (bind _self self)
  (bind _returnvalue (Class|GameFunctionLibrary|GetFSDGameMode _self))
  (for _array_element (Variables|/Script/FSD.FSDGameMode|GetPlayerControllers _returnvalue)
    (CallFunction|SpawnReplicatedActorforPlayerController _array_element))
  (EventDispatchers|BindEventtoOnPlayerLoggedin _returnvalue (EventDispatchers|CreateEvent :!event SpawnReplicatedActorforPlayerController)))

(fn SpawnReplicatedActorforPlayerController
  (params (Player%20Controller :type FSD%20Player%20Controller%20Object%20Reference))
  (Game|SpawnActorfromClass "/Game/StyleMeter/BP_StyleMeterReplicatedActor.BP_StyleMeterReplicatedActor_C" (Math|Transform|MakeTransform "0, 0, 0") "Undefined" Player%20Controller self Player%20Controller 0))