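; Master actor for a handshake test mod that registers the mod and creates a replicated actor per registered player controller.
; On BeginPlay it registers its handshake ID in clientside storage and, on the server, registers itself as the awaiting mod in hostside storage.
; The registration event then spawns a BP_HandshakingModReplicatedActor with that controller as owner.
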(event EventBeginPlay
  (CallFunction|HandleBeginPlay))

(event Collision|EventActorBeginOverlap
  (params (OtherActor :type Actor%20Object%20Reference)))

(event EventTick
  (params (DeltaSeconds :type Float%20%28single-precision%29)))

(event EventOnModRegisteredforPlayerController
  (params (Player%20Controller :type FSD%20Player%20Controller%20Object%20Reference))
  (CallFunction|SpawnReplicatedActorforController Player%20Controller))

(fn ConstructionScript)

(fn HandleBeginPlay
  (Default|RegisterLocalMod (Variables|Default|GetClientside%20Registered%20Mods%20Storage) (Variables|Default|GetHandshake%20Mod%20ID))
  (if (Networking|IsServer)
    (Default|RegisterHostsideMod (Variables|Default|GetHostside%20Listening%20Mods%20Storage) (Variables|Default|GetHandshake%20Mod%20ID) self)))

(fn SpawnReplicatedActorforController
  (params (Player%20Controller :type FSD%20Player%20Controller%20Object%20Reference))
  (Game|SpawnActorfromClass "/Game/HandshakeTestMod/BP_HandshakingModReplicatedActor.BP_HandshakingModReplicatedActor_C" (Math|Transform|MakeTransform "0, 0, 0") "Undefined" Player%20Controller Player%20Controller 0))