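; BP_HandshakingModReplicatedActor is an actor that registers the handshake test mod's UI page for the local player.
; On BeginPlay it checks whether its owning player controller is local.
; If so, it creates a UI_HandshakingModPage widget, stores it as ModHubPage and passes it to AddPage.
; Overlap and Tick are disabled, and the construction script only calls its parent.
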(event EventBeginPlay
  (CallFunction|HandleBeginPlay))

(event Collision|EventActorBeginOverlap
  (params (OtherActor :type Actor%20Object%20Reference))
  (|CallParentFunction OtherActor) ; This node is disabled and will not be called.\nDrag off pins to build functionality.
)

(event EventTick
  (params (DeltaSeconds :type Float%20%28single-precision%29))
  (|CallParentFunction DeltaSeconds) ; This node is disabled and will not be called.\nDrag off pins to build functionality.
)

(fn ConstructionScript
  (|CallParentFunction))

(fn HandleBeginPlay
  (if (Pawn|IsLocalPlayerController (Variables|Default|GetOwning%20Player%20Controller))
    (bind _returnvalue (UserInterface|CreateWidget "/Game/HandshakeTestMod/UI_HandshakingModPage.UI_HandshakingModPage_C"))
    (bind _output_get (Variables|Default|SetMod%20Hub%20Page _returnvalue))
    (CallFunction|AddPage _output_get)))