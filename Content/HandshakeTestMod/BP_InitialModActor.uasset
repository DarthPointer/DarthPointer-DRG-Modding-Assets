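; Initial actor for the HandshakeTestMod, which registers the mod's UI page and offers spawning of the handshaking mod master actor.
; On BeginPlay it creates a UI_InitialModPage widget, passes it to AddPage and binds an event to the page's spawn button click.
; A separate function, the apparent target of that binding, spawns BP_HandshakingModMasterActor at the world origin.
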(event EventBeginPlay
  (CallFunction|HandleBeginPlay))

(event Collision|EventActorBeginOverlap
  (params (OtherActor :type Actor%20Object%20Reference))
  (|CallParentFunction OtherActor) ; This node is disabled and will not be called.\nDrag off pins to build functionality.
)

(event EventTick
  (params (DeltaSeconds :type Float%20%28single-precision%29))
  (|CallParentFunction DeltaSeconds) ; This node is disabled and will not be called.\nDrag off pins to build functionality.
)

(fn ConstructionScript
  (|CallParentFunction))

(fn HandleBeginPlay
  (bind _returnvalue (UserInterface|CreateWidget "/Game/HandshakeTestMod/UI_InitialModPage.UI_InitialModPage_C"))
  (bind _output_get (Variables|Default|SetMod%20Hub%20Page _returnvalue))
  (CallFunction|AddPage _output_get)
  (EventDispatchers|BindEventtoOnClicked (Variables|/Game/HandshakeTestMod/UI_InitialModPage.UI_InitialModPage_C|GetSpawnHandshakingModmasterActor _output_get) (EventDispatchers|CreateEvent :!event SpawnHandshakingModMasterActor)))

(fn SpawnHandshakingModMasterActor
  (Game|SpawnActorfromClass "/Game/HandshakeTestMod/BP_HandshakingModMasterActor.BP_HandshakingModMasterActor_C" (Math|Transform|MakeTransform "0, 0, 0") "Undefined" 0 0))