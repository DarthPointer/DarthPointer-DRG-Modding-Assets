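; Example vanity mod actor that creates a mod page widget and reports how the parent's begin-play handling affects the EngieSet armor item count.
; HandleBeginPlay adds the page to the viewport and the Pages array, then writes the armor count to its text fields before and after calling the parent implementation.
; GetModPages returns that array, while GetModInfo returns blank name, author and version.
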(event EventBeginPlay
  (|CallParentFunction) ; This node is disabled and will not be called.\nDrag off pins to build functionality.
)

(event Collision|EventActorBeginOverlap
  (params (OtherActor :type Actor%20Object%20Reference))
  (|CallParentFunction OtherActor) ; This node is disabled and will not be called.\nDrag off pins to build functionality.
)

(event EventTick
  (params (DeltaSeconds :type Float%20%28single-precision%29))
  (|CallParentFunction DeltaSeconds) ; This node is disabled and will not be called.\nDrag off pins to build functionality.
)

(fn ConstructionScript
  (|CallParentFunction))

(fn HandleBeginPlay
  (bind _returnvalue (UserInterface|CreateWidget "/Game/VanityModExample/Page.Page_C"))
  (bind _output_get (Variables|Default|SetPage _returnvalue))
  (UserInterface|Viewport|AddtoViewport _output_get 0)
  (Utilities|Array|Add (Variables|Default|GetPages) _output_get)
  (Rendering|Components|TextRender|SetText (Variables|/Game/VanityModExample/Page.Page_C|GetArmorsBefore (Variables|Default|GetPage)) (Utilities|Text|ToText(Integer) (Utilities|Array|Length (Variables|/Script/FSD.CharacterVanityItems|GetArmorItems (LocalVariables|GetEngie%20Set)))))
  (|CallParentFunction)
  (Rendering|Components|TextRender|SetText (Variables|/Game/VanityModExample/Page.Page_C|GetArmorsAfter (Variables|Default|GetPage)) (Utilities|Text|ToText(Integer) (Utilities|Array|Length (Variables|/Script/FSD.CharacterVanityItems|GetArmorItems (LocalVariables|GetEngie%20Set))))))

(fn GetModInfo
  (return "" "" ""))

(fn GetModPages
  (return (Variables|Default|GetPages)))